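; BP_U_Terminal is the Terminal program in the Unix flavor of an in-game operating system.
; It acts as a thin bridge, casting its program widget to WBP_Unix_Terminal and forwarding each command event to it.
; Command messages and completion errors pass through to the widget, while root password and user continue requests make it create the matching prompts.
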(event EventPromptRootPassword
  (Default|CreateRootCommandPrompt (.AsWBP%20Unix%20Terminal (Utilities|Casting|CastToWBP_Unix_Terminal (Variables|Default|GetProgramWidget)))))

(event EventMessageReceivedfromCommand
  (params (CmdMsg :type Text%20%28by%20ref%29) (CmdMsgType :type EOperatingSystemTerminalMessageType%20Enum%20%28by%20ref%29 :default "Normal"))
  (Default|OnMessageReceived (.AsWBP%20Unix%20Terminal (Utilities|Casting|CastToWBP_Unix_Terminal (Variables|Default|GetProgramWidget))) CmdMsg CmdMsgType))

(event EventCommandFinished
  (params (ErrorMessage :type Generic%20Error%20Structure%20%28by%20ref%29))
  (Default|OnCommandFinished (.AsWBP%20Unix%20Terminal (Utilities|Casting|CastToWBP_Unix_Terminal (Variables|Default|GetProgramWidget))) ErrorMessage))

(event EventPromptUserContinue
  (Default|CreateUserContinuePrompt (.AsWBP%20Unix%20Terminal (Utilities|Casting|CastToWBP_Unix_Terminal (Variables|Default|GetProgramWidget)))))