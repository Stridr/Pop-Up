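; Terminal "help" command for the in-game operating system, showing the description of another command.
; ProcessCommand runs InternalDisplayHelp and passes the resulting error to FinishCommand.
; The helper requires exactly one parameter, looks it up through ParentTerminal.GetCommand and sends that command's description to the terminal as a normal message.
; A wrong parameter count yields a generic help error, and a failed lookup returns the terminal's own error.
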(event EventProcessCommand
  (params (Command :type String) (bHasRootPermission :type Boolean))
  (bind _returnvalue (CallFunction|InternalDisplayHelp))
  (Class|OperatingSystemTerminalCommand|FinishCommand _returnvalue))

(fn InternalDisplayHelp
  (bind _commandparameters (Variables|Default|GetCommandParameters))
  (bind _parentterminal (Variables|Default|GetParentTerminal))
  (bind _commandparameters_2 (Variables|Default|GetCommandParameters))
  (bind _returnvalue (Utilities|Array|Length _commandparameters))
  (bind _output (Utilities|Array|Get(acopy) _commandparameters_2))
  (bind (_outerror _returnvalue_2) (Class|OperatingSystemTerminal|GetCommand _parentterminal _output))
  (Utilities|FlowControl|Sequence
    (:then_0
      (if (> _returnvalue 1)
        (bind _returnvalue_3 (Class|OperatingSystemStatics|CreateGenericError (Utilities|Text|MakeLiteralText "ERR_TERMINAL_HELP") (Utilities|Text|FormatText "Too many parameters for {Name} command." (Class|OperatingSystemTerminalCommand|GetMainCommand))))
        (LocalVariables|SetLocal_Error _returnvalue_3)
        (elif (== _returnvalue 0)
          (bind _returnvalue_4 (Class|OperatingSystemStatics|CreateGenericError (Utilities|Text|MakeLiteralText "ERR_TERMINAL_HELP") (Utilities|Text|FormatText "Provide a command as parameter to {Name} to show its description." (Class|OperatingSystemTerminalCommand|GetMainCommand))))
          (LocalVariables|SetLocal_Error _returnvalue_4)
          (else
            (bind _output_get (LocalVariables|SetLocal_Error _outerror))
            (if (not (.bIsValid (Utilities|Struct|BreakGenericError _output_get)))
              (bind _output_get_2 (LocalVariables|SetLocal_Command _returnvalue_2))
              (Class|OperatingSystemTerminalCommand|NotifyTerminal (Class|OperatingSystemTerminalCommand|GetCommandDescription _output_get_2) "Normal"))))))
    (:then_1
      (return (LocalVariables|GetLocal_Error)))))