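; Terminal command Blueprint for cd, which changes the current path of the parent terminal in an in-game operating system.
; ProcessCommand runs an internal function and passes its resulting error to FinishCommand.
; That function expects exactly one parameter and hands it to the terminal's ChangeCurrentPath.
; A failed path change, missing parameter or excess parameters each produce a generic command error with a matching message.
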(event EventProcessCommand
  (params (Command :type String) (bHasRootPermission :type Boolean))
  (bind _returnvalue (CallFunction|InternalProcessCdCommand))
  (Class|OperatingSystemTerminalCommand|FinishCommand _returnvalue))

(fn InternalProcessCdCommand
  (bind _returnvalue (Class|OperatingSystemTerminalCommand|GetMainCommand))
  (Utilities|FlowControl|Sequence
    (:then_0
      (bind _output_get (LocalVariables|SetLocal_FlagCount (Utilities|Array|Length (Variables|Default|GetCommandParameters))))
      (if (== _output_get 1)
        (bind _returnvalue_2 (Class|OperatingSystemTerminal|ChangeCurrentPath (Variables|Default|GetParentTerminal) (Utilities|Array|Get(acopy) (Variables|Default|GetCommandParameters))))
        (if (not _returnvalue_2)
          (bind _returnvalue_3 (Class|OperatingSystemStatics|CreateGenericError (Utilities|Text|MakeLiteralText "ERR_CMD") (Utilities|Text|MakeLiteralText "No such directory.")))
          (LocalVariables|SetLocal_Error _returnvalue_3))
        (else
          (bind _returnvalue_4 (Class|OperatingSystemStatics|CreateGenericError (Utilities|Text|MakeLiteralText "ERR_CMD") (select (== (LocalVariables|GetLocal_FlagCount) 0) (Utilities|Text|FormatText "Missing parameter for {CmdName} command." _returnvalue) (Utilities|Text|FormatText "Too many parameters for {CmdName} command." _returnvalue))))
          (LocalVariables|SetLocal_Error _returnvalue_4))))
    (:then_1
      (return (LocalVariables|GetLocal_Error)))))