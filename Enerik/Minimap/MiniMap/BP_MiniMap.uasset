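; BP_MiniMap is an actor that shows the player minimap and keeps its material data up to date.
; On BeginPlay it creates the W_Minimap widget and adds it to the viewport.
; Every Tick it writes the player character's location and yaw, wrapped to positive and normalized to a 0–1 turn, into the MP_MiniMap Material Parameter Collection.
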(event EventBeginPlay
  (bind _returnvalue (UserInterface|CreateWidget "/Game/Enerik/Minimap/MiniMap/W_Minimap.W_Minimap_C"))
  (UserInterface|Viewport|AddtoViewport _returnvalue 0))

(event Collision|EventActorBeginOverlap
  (params (OtherActor :type Actor%20Object%20Reference)))

(event EventTick
  (params (DeltaSeconds :type Float%20%28single-precision%29))
  (bind _returnvalue (Game|GetPlayerCharacter 0))
  (bind _returnvalue_2 (Transformation|GetActorRotation _returnvalue))
  (bind _yaw (Math|Rotator|BreakRotator _returnvalue_2))
  (Rendering|Material|SetVectorParameterValue "/Game/Enerik/Minimap/MiniMap/MP_MiniMap.MP_MiniMap" "PlayerLocation" (Math|Conversions|ToLinearColor(Vector) (Transformation|GetActorLocation _returnvalue)) :!class /Script/Engine.KismetMaterialLibrary)
  (Rendering|Material|SetScalarParameterValue "/Game/Enerik/Minimap/MiniMap/MP_MiniMap.MP_MiniMap" "PlayerYaw" (/ (Math|Float|SelectFloat (+ _yaw 3.6e+02) _yaw (< _yaw 0.0)) 3.6e+02) :!class /Script/Engine.KismetMaterialLibrary))

(fn ConstructionScript)